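; Collectible coin Blueprint that bobs up and down until a BP_2DCharacter picks it up.
; Overlapping its collision calls AddCoin on the character, plays a click sound at the coin's location and destroys the actor.
; Tick drives the bobbing with a small fixed per-frame local offset, whose direction a Delay and FlipFlop reverse about every half second, so travel distance depends on frame rate.
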(event `self.Collision.OnComponentBeginOverlap`
  (params (OverlappedComponent :type "PrimitiveComponent Object Reference") (OtherActor :type "Actor Object Reference") (OtherComp :type "PrimitiveComponent Object Reference") (OtherBodyIndex :type Integer) (bFromSweep :type Boolean) (SweepResult :type "HitResult Structure (by ref)"))
  (bind _asbp_2dcharacter (cast `/Game/Blueprints/BP_2DCharacter` OtherActor))
  (`/Game/Blueprints/BP_2DCharacter.AddCoin` _asbp_2dcharacter)
  (`self.PlaySound`))

(event `PlaySound`
  (`GameplayStatics.PlaySoundAtLocation` "/Engine/VREditor/Sounds/UI/Click_on_Button_Cue.Click_on_Button_Cue" (`self.K2_GetActorLocation`) (struct) 1.0 1.0 0.0 null null null null)
  (`self.K2_DestroyActor`))

(event `self.ReceiveTick`
  (params (DeltaSeconds :type "Float (single-precision)"))
  ;[1 1 1] Coin go up and down
  (`|ExecutionSequence`
    (:`then_0`
      (`KismetSystemLibrary.Delay` 0.5)
      (`/Engine/EditorBlueprintResources/StandardMacros.FlipFlop`
        (:`A`
          (set `self.dir` true))
        (:`B`
          (bind _output_get (set `self.dir` false)))))
    (:`then_1`
      (if (`self.dir`)
        (`self.K2_AddActorLocalOffset` (0.0 0.0 0.1))
        (else
          (`self.K2_AddActorLocalOffset` (0.0 0.0 -0.1)))))))

(fn `UserConstructionScript`)