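; P1_Controller is a player controller that drives the 2D character for player one.
; On BeginPlay it casts player character 0 to BP_2DCharacter, stores the reference and possesses it.
; The left/right and forward/backward input axes pass their values to the character's movement functions.
; An unconnected GetAllActorsOfClass lookup is left in the graph unused.
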(event `self.ReceiveBeginPlay`
  (bind _asbp_2dcharacter (cast `/Game/Blueprints/BP_2DCharacter` (`GameplayStatics.GetPlayerCharacter` 0)))
  (bind _output_get (set `self.As BP 2DCharacter` _asbp_2dcharacter))
  (`self.Possess` _output_get))

(event `InputAxis|Move_LeftRight`
  (params (AxisValue :type "Float (single-precision)"))
  (`/Game/Blueprints/BP_2DCharacter.MoveLeftRight` (`self.As BP 2DCharacter`) AxisValue))

(event `InputAxis|Foward_Backward`
  (params (AxisValue :type "Float (single-precision)"))
  (`/Game/Blueprints/BP_2DCharacter.MoveForwardBackward` (`self.As BP 2DCharacter`) AxisValue))

(fn `UserConstructionScript`)